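; Lantern actor whose point light switches on while the TopDownCharacter is near it.
; Overlap events on a Sphere component set the light intensity to a fixed bright value on entry and to zero on exit, ignoring other actors.
; The construction script removes the Cube component unless Standing is set and starts the light dark unless StartOn is set.
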(event `self.Sphere.OnComponentBeginOverlap`
  (params (OverlappedComponent :type "PrimitiveComponent Object Reference") (OtherActor :type "Actor Object Reference") (OtherComp :type "PrimitiveComponent Object Reference") (OtherBodyIndex :type Integer) (bFromSweep :type Boolean) (SweepResult :type "HitResult Structure (by ref)"))
  (cast `/Game/TopDownBP/Blueprints/TopDownCharacter` OtherActor)
  (`LightComponent.SetIntensity` (`self.PointLight`) 10000.0))

(event `self.Sphere.OnComponentEndOverlap`
  (params (OverlappedComponent :type "PrimitiveComponent Object Reference") (OtherActor :type "Actor Object Reference") (OtherComp :type "PrimitiveComponent Object Reference") (OtherBodyIndex :type Integer))
  (cast `/Game/TopDownBP/Blueprints/TopDownCharacter` OtherActor)
  (`LightComponent.SetIntensity` (`self.PointLight`) 0.0))

(fn `UserConstructionScript`
  (if (not (`self.Standing`))
    (`ActorComponent.K2_DestroyComponent` (`self.Cube`)))
  (if (not (`self.Start On`))
    (`LightComponent.SetIntensity` (`self.PointLight`) 0.0)))