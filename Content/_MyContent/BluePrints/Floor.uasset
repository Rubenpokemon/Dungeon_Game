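; Floor actor that builds a rectangular grid of cube tiles, sized by its X and Y variables.
; The Construction Script runs nested loops, adding a scaled static mesh component per cell and stepping SpawnX and SpawnY to place the tiles at even intervals.
; The event graph holds only disabled placeholder events, so the actor has no runtime logic of its own.
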(fn `UserConstructionScript`
  (locals (`Spawn X` :type "Float (double-precision)") (`Spawn Y` :type "Float (double-precision)"))
  (for _ (range 1 (+ (`self.X`) 1))
    (for _ (range 1 (+ (`self.Y`) 1))
      (bind _returnvalue (`AddComponent|NODE_AddStaticMeshComponent-0`))
      (`StaticMeshComponent.SetStaticMesh` _returnvalue "/Game/Geometry/Meshes/1M_Cube.1M_Cube")
      (`SceneComponent.SetRelativeScale3D` _returnvalue (2.5 2.5 1.0))
      (`SceneComponent.K2_SetRelativeLocation` _returnvalue (`KismetMathLibrary.MakeVector` (`local.Spawn X`) (`local.Spawn Y`)) false false)
      (set `local.Spawn Y` (+ (`local.Spawn Y`) 250.0)))
    (set `local.Spawn X` (+ (`local.Spawn X`) 250.0))
    (set `local.Spawn Y` 0.0)))