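; Laser shot actor whose size and damage scale with its FirePower value.
; Shortly after BeginPlay, it scales its Cube from FirePower, slightly longer on Y.
; Cube overlaps ignore the player pawn; actors tagged Enemy are cast to Base_Enemy and take FirePower-based damage.
; The laser destroys itself after a brief delay on hitting an enemy or any other non-player actor, but persists if that cast fails.
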(event `self.ReceiveBeginPlay`
  (bind _returnvalue (+ (/ (`KismetMathLibrary.Conv_IntToDouble` (`self.FirePower`)) 25.0) 0.06))
  (`KismetSystemLibrary.Delay` 0.01)
  (`SceneComponent.SetRelativeScale3D` (`self.Cube`) (`KismetMathLibrary.MakeVector` _returnvalue (+ _returnvalue 0.24) _returnvalue)))

(event `self.Cube.OnComponentBeginOverlap`
  (params (OverlappedComponent :type "PrimitiveComponent Object Reference") (OtherActor :type "Actor Object Reference") (OtherComp :type "PrimitiveComponent Object Reference") (OtherBodyIndex :type Integer) (bFromSweep :type Boolean) (SweepResult :type "HitResult Structure (by ref)"))
  (if (!= OtherActor (`GameplayStatics.GetPlayerPawn` 0))
    (if (`self.ActorHasTag` OtherActor "Enemy")
      (bind _asbase_enemy (cast `/Game/_MyContent/BluePrints/Base_Enemy` OtherActor))
      (`/Game/_MyContent/BluePrints/Base_Enemy.Damage` _asbase_enemy (+ (* (`self.FirePower`) 50.0) 50.0)))
    (`KismetSystemLibrary.Delay` 0.01)
    (`self.K2_DestroyActor`)))

(fn `UserConstructionScript`)