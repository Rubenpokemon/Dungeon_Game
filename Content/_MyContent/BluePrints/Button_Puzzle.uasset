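; Five-button "Lights Out" style puzzle actor that opens a linked Locked_Gate when all buttons are lit.
; Clicking a button component uses its numeric name as an index to toggle the materials of that button and its neighbours.
; After each press it counts lit buttons to check for a win.
; The construction script shuffles button positions and scrambles the starting state with random presses, so neighbours follow index rather than layout.
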(event `self.0.OnClicked`
  (params (TouchedComponent :type "PrimitiveComponent Object Reference") (ButtonPressed :type "Key Structure"))
  (`self.Press Button` (`KismetStringLibrary.Conv_StringToInt` (`KismetSystemLibrary.GetObjectName` TouchedComponent))))

(event `self.1.OnClicked`
  (params (TouchedComponent :type "PrimitiveComponent Object Reference") (ButtonPressed :type "Key Structure"))
  (`self.Press Button` (`KismetStringLibrary.Conv_StringToInt` (`KismetSystemLibrary.GetObjectName` TouchedComponent))))

(event `self.2.OnClicked`
  (params (TouchedComponent :type "PrimitiveComponent Object Reference") (ButtonPressed :type "Key Structure"))
  (`self.Press Button` (`KismetStringLibrary.Conv_StringToInt` (`KismetSystemLibrary.GetObjectName` TouchedComponent))))

(event `self.3.OnClicked`
  (params (TouchedComponent :type "PrimitiveComponent Object Reference") (ButtonPressed :type "Key Structure"))
  (`self.Press Button` (`KismetStringLibrary.Conv_StringToInt` (`KismetSystemLibrary.GetObjectName` TouchedComponent))))

(event `self.4.OnClicked`
  (params (TouchedComponent :type "PrimitiveComponent Object Reference") (ButtonPressed :type "Key Structure"))
  (`self.Press Button` (`KismetStringLibrary.Conv_StringToInt` (`KismetSystemLibrary.GetObjectName` TouchedComponent))))

(fn `Check Buttons Materials`
  (locals (`Buttons On` :type Integer))
  (for _array_element (`self.Buttons`)
    (if (== (`PrimitiveComponent.GetMaterial` _array_element 0) (`self.Material On`))
      (set `local.Buttons On` (+ (`local.Buttons On`) 1))))
  (if (== (`local.Buttons On`) 5)
    (`self.Win`)))

(fn `Press Button`
  (params (Button :type Integer))
  (locals (`Button - 1` :type Integer :default -1) (`Button + 1` :type Integer :default -1) (`Button =` :type Integer))
  (bind _button__ (`local.Button =`))
  (set `local.Button =` Button)
  (if (== Button 0)
    (set `local.Button + 1` 1)
    (elif (< Button 4)
      (set `local.Button + 1` (+ _button__ 1))
      (set `local.Button - 1` (- _button__ 1))
      (else
        (set `local.Button - 1` 3))))
  (`self.Swap Materials` (`|MakeArray` (`local.Button =`) (`local.Button + 1`) (`local.Button - 1`))))

(fn `Swap Materials`
  (params (Array :type "Array of Integer"))
  (locals (Cube :type "StaticMeshComponent Object Reference"))
  (bind _cube (`local.Cube`))
  (for _array_element Array
    (if (!= _array_element -1)
      (bind _output (`|GetArrayItem` (`self.Buttons`) _array_element))
      (set `local.Cube` _output)
      (if (== (`PrimitiveComponent.GetMaterial` _output 0) "/Game/_MyContent/Materials/Black.Black")
        (`PrimitiveComponent.SetMaterial` _cube 0 (`self.Material On`))
        (else
          (`PrimitiveComponent.SetMaterial` _cube 0 (`self.Material Off`))))))
  (`self.Check Buttons Materials`))

(fn `UserConstructionScript`
  (locals (`Buttons 2` :type "Array of StaticMeshComponent Object Reference") (`Spawn X` :type "Float (double-precision)" :default -400.0))
  (bind _output_get (set `self.Buttons` (`|MakeArray` (`self.0`) (`self.1`) (`self.2`) (`self.3`) (`self.4`))))
  ;[1 1 1] Shuffle Blocks
  (bind _output_get_2 (set `local.Buttons 2` _output_get))
  (`KismetArrayLibrary.Array_Shuffle` _output_get_2)
  (for (_array_element _array_index) (`local.Buttons 2`)
    (`SceneComponent.K2_SetRelativeLocation` _array_element (`|GetArrayItem` (`self.Vectors`) _array_index) false false))
  (for _ (range (+ (`KismetMathLibrary.RandomIntegerInRange` 6 9) 1))
    (`self.Press Button` (`KismetMathLibrary.RandomIntegerInRange` 0 4))))

(fn `Win`
  (bind _gate (`self.Gate`))
  (if (`KismetSystemLibrary.IsValid` _gate)
    (bind _aslocked_gate (cast `/Game/_MyContent/BluePrints/Locked_Gate` _gate))
    (`/Game/_MyContent/BluePrints/Locked_Gate.Open Gate` _aslocked_gate)))