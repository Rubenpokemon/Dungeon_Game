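; Arena gate actor that seals when the TopDownCharacter enters its active trigger, runs enemy waves, then reopens.
; Timelines slide the Cube vertically, and closing and opening propagate to linked OtherGates.
; Each wave spawns staggered AI at shuffled spawn points, then polls the Enemies array until empty.
; WaveSize grows by one per wave until Waves reaches zero, when the gate reopens and disables Cube collision.
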(event `Close Gate`
  (bind (_direction _close) (`Timeline|Timeline_1` :!via `PlayFromStart`)
    (:`Update`
      (`SceneComponent.K2_SetRelativeLocation` (`self.Cube`) (`KismetMathLibrary.MakeVector` 0.0 0.0 _close) false false))))

(event `self.Trigger.OnComponentBeginOverlap`
  (params (OverlappedComponent :type "PrimitiveComponent Object Reference") (OtherActor :type "Actor Object Reference") (OtherComp :type "PrimitiveComponent Object Reference") (OtherBodyIndex :type Integer) (bFromSweep :type Boolean) (SweepResult :type "HitResult Structure (by ref)"))
  (bind _other_gates (`self.Other Gates`))
  (if (`self.Active`)
    (cast `/Game/TopDownBP/Blueprints/TopDownCharacter` OtherActor)
    (if (not (`self.Gate Closed`))
      (set `self.Gate Closed` true)
      (bind (_direction _close) (`Timeline|Close_Gate` :!via `PlayFromStart`)
        (:`Update`
          (`SceneComponent.K2_SetRelativeLocation` (`self.Cube`) (`KismetMathLibrary.MakeVector` 0.0 0.0 _close) false false))
        (:`Finished`
          (`self.New Wave`)
          (if (not (== (`KismetArrayLibrary.Array_Length` _other_gates) 0))
            (for _array_element _other_gates
              (bind _asgate (cast `/Game/_MyContent/BluePrints/Gate` _array_element))
              (`self.Close Gate` _asgate))))))))

(event `New Wave`
  (bind _enemies (`self.Enemies`))
  (bind _output_get (set `self.Enemies To Spawn` (`self.Wave Size`)))
  (if (> _output_get 0) :!label _label
    (`self.Spawn_Enemy`)
    (`KismetSystemLibrary.Delay` 0.2)
    (set `self.Enemies To Spawn` (- (`self.Enemies To Spawn`) 1))
    (goto _label)
    (else
      (`KismetSystemLibrary.Delay` 1.0 :!label _label_2)
      (for _array_element _enemies
        (if (not (`KismetSystemLibrary.IsValid` _array_element))
          (`KismetArrayLibrary.Array_RemoveItem` (`self.Enemies`) _array_element)))
      (if (>= (`KismetArrayLibrary.Array_Length` _enemies) 1)
        (goto _label_2)
        (else
          (bind _result (`/Engine/EditorBlueprintResources/StandardMacros.IncrementInt` (`self.Wave Size`))
            (:`  `
              (set `self.Wave Size` _result)
              (bind _result_2 (`/Engine/EditorBlueprintResources/StandardMacros.DecrementInt` (`self.Waves`))
                (:`  `
                  (bind _output_get_2 (set `self.Waves` _result_2))
                  (if (== _output_get_2 0)
                    (`self.Open Gate`)
                    (else
                      (`self.New Wave`))))))))))))

(event `Open Gate`
  (bind _other_gates (`self.Other Gates`))
  (bind (_direction _close) (`Timeline|Timeline_0` :!via `ReverseFromEnd`)
    (:`Update`
      (`SceneComponent.K2_SetRelativeLocation` (`self.Cube`) (`KismetMathLibrary.MakeVector` 0.0 0.0 _close) false false))
    (:`Finished`
      (`PrimitiveComponent.SetCollisionEnabled` (`self.Cube`) "NoCollision")
      (if (not (== (`KismetArrayLibrary.Array_Length` _other_gates) 0))
        (for _array_element _other_gates
          (bind _asgate (cast `/Game/_MyContent/BluePrints/Gate` _array_element))
          (`self.Open Gate` _asgate))))))

(fn `Get Random SpawnPoint Location`
  (returns (Vector :type "Vector Structure"))
  (bind _spawnpoints (`self.SpawnPoints`))
  (`KismetArrayLibrary.Array_Shuffle` _spawnpoints)
  (return (`self.K2_GetActorLocation` (`|GetArrayItem` _spawnpoints))))

(fn `Spawn_Enemy`
  (bind _vector (`self.Get Random SpawnPoint Location`))
  (bind _returnvalue (`AIBlueprintHelperLibrary.SpawnAIFromClass` "/Game/_MyContent/BluePrints/Enemy.Enemy_C" null _vector (struct) true null))
  (`KismetArrayLibrary.Array_Add` (`self.Enemies`) _returnvalue))

(fn `UserConstructionScript`
  (locals (Max_X :type "Float (double-precision)") (Min_X :type "Float (double-precision)") (Max_Y :type "Float (double-precision)") (Min_Y :type "Float (double-precision)"))
  (if (and (`self.Gate Closed`) (not (`self.Active`)))
    (`ActorComponent.K2_DestroyComponent` (`self.Trigger`))))