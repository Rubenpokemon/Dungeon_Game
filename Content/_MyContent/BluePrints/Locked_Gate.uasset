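; Locked gate Blueprint that opens when clicked if the player's TopDownCharacter carries the required item.
; A click on the Box checks the character's Items for ItemNeeded, then plays the Open timeline to move the mesh along relative Z.
; The Box is destroyed once the timeline finishes.
; Its collision is disabled in the Construction Script and enabled at BeginPlay, after the player cast succeeds.
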(event `self.ReceiveBeginPlay`
  (bind _astop_down_character (cast `/Game/TopDownBP/Blueprints/TopDownCharacter` (`GameplayStatics.GetPlayerPawn` 0)))
  (set `self.Player` _astop_down_character)
  (`PrimitiveComponent.SetCollisionEnabled` (`self.Box`) "QueryAndPhysics"))

(event `self.Box.OnClicked`
  (params (TouchedComponent :type "PrimitiveComponent Object Reference") (ButtonPressed :type "Key Structure"))
  (if (`KismetArrayLibrary.Array_Contains` (`/Game/TopDownBP/Blueprints/TopDownCharacter.Items` (`self.Player`)) (`self.Item Needed`))
    (`self.Open Gate`)))

(event `Open Gate`
  (bind (_direction _newtrack_0) (`Timeline|Open` :!via `PlayFromStart`)
    (:`Update`
      (`SceneComponent.K2_SetRelativeLocation` (`self.Mesh`) (`KismetMathLibrary.MakeVector` 0.0 0.0 _newtrack_0) false false))
    (:`Finished`
      (`ActorComponent.K2_DestroyComponent` (`self.Box`)))))

(fn `UserConstructionScript`
  (`PrimitiveComponent.SetCollisionEnabled` (`self.Box`) "NoCollision"))