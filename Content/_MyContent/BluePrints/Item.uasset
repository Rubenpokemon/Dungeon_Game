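; Clickable world item that the player picks up into the TopDownCharacter.
; On BeginPlay it caches the player pawn as a TopDownCharacter.
; Clicking its Cube within a fixed distance of the player passes ItemType to the character's AddItem and destroys the actor.
; The construction script sets the actor's Tags from a local variable.
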(event `self.ReceiveBeginPlay`
  (bind _astop_down_character (cast `/Game/TopDownBP/Blueprints/TopDownCharacter` (`GameplayStatics.GetPlayerPawn` 0)))
  (set `self.Player` _astop_down_character))

(event `self.Cube.OnClicked`
  (params (TouchedComponent :type "PrimitiveComponent Object Reference") (ButtonPressed :type "Key Structure"))
  (if (<= (`KismetMathLibrary.VSize` (- (`self.K2_GetActorLocation` (`self.Player`)) (`SceneComponent.K2_GetComponentLocation` (`self.DefaultSceneRoot`)))) 200.0)
    (`/Game/TopDownBP/Blueprints/TopDownCharacter.Add Item` (`self.Player`) (`self.Item Type`))
    (`self.K2_DestroyActor`)))

(fn `UserConstructionScript`
  (locals (NewLocalVar_0 :type "Array of Name"))
  (set `self.Tags` (`local.NewLocalVar_0`)))