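; Enemy laser projectile actor that damages the player on contact.
; When its Cube component begins overlapping the player pawn, it calls Hit on the TopDownCharacter with its Damage and destroys itself after a tiny delay.
; Overlaps with other actors also destroy it, except those tagged Enemy, which it ignores.
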(event `self.Cube.OnComponentBeginOverlap`
  (params (OverlappedComponent :type "PrimitiveComponent Object Reference") (OtherActor :type "Actor Object Reference") (OtherComp :type "PrimitiveComponent Object Reference") (OtherBodyIndex :type Integer) (bFromSweep :type Boolean) (SweepResult :type "HitResult Structure (by ref)"))
  (if (== OtherActor (`GameplayStatics.GetPlayerPawn` 0))
    (bind _astop_down_character (cast `/Game/TopDownBP/Blueprints/TopDownCharacter` OtherActor))
    (`/Game/TopDownBP/Blueprints/TopDownCharacter.Hit` _astop_down_character (`self.Damage`))
    (`KismetSystemLibrary.Delay` 0.01)
    (`self.K2_DestroyActor`)
    (elif (not (`self.ActorHasTag` OtherActor "Enemy"))
      (`KismetSystemLibrary.Delay` 0.01)
      (`self.K2_DestroyActor`))))

(fn `UserConstructionScript`)