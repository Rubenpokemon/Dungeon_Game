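; One enemy Blueprint covers five types in a top-down game: melee, laser shooter, healer, suicide-diving sapling, and spawner of saplings.
; Construction resolves the type (an unset one uses weighted chances, currently with a hardcoded roll) and SetType applies mesh and stats.
; Tick drives AIMoveTo chasing, or retreat for shooter and spawner, attacking in range or near walls.
; Attacks use timelines, delays and an Attacking lock; health updates a widget bar.
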(event `self.ReceiveBeginPlay`
  (set `self.Player` (`GameplayStatics.GetPlayerPawn` 0))
  (bind _ashealth_bar (cast `/Game/_MyContent/UI/HealthBar` (`WidgetComponent.GetUserWidgetObject` (`self.Widget`))))
  (bind _output_get (set `self.Health Bar` _ashealth_bar))
  (set `/Game/_MyContent/UI/HealthBar.Health Percent` 1.0 _output_get)
  (`self.Set Type`))

(event `Melee Movement`
  (if (`self.Attacking`)
    _
    (elif (`self.Player In Attacking Range`)
      (`self.Attack`)
      (else
        (`self.Move Foward`)))))

(event `Ranged Movement`
  (if (not (`self.Player In Running Range`))
    (if (`self.Attacking`)
      _
      (elif (`self.Player In Attacking Range`)
        (`self.Attack` :!label _label)
        (else
          (`self.Move Foward`))))
    (else
      (bind _true (`self.Objects Around`))
      (if _true
        (goto _label)
        (else
          (`self.Run Away`))))))

(event `Move Foward`
  (`|AIMoveTo` self (0.0 0.0 0.0) (`self.Player`)))

(event `self.ReceiveTick`
  (params (DeltaSeconds :type "Float (single-precision)"))
  (switch `int` (`self.Type`)
    (:`0`
      (`self.Melee Movement` :!label _label_2))
    (:`1`
      (`self.Ranged Movement` :!label _label_3))
    (:`2`
      (goto _label_2))
    (:`3`
      (goto _label_2))
    (:`4`
      (goto _label_3))))

(event `Run Away`
  (bind _returnvalue (`self.K2_GetActorLocation`))
  (`|AIMoveTo` self (`KismetMathLibrary.MakeVector` (.x (+ _returnvalue (* (`KismetMathLibrary.GetForwardVector` (`KismetMathLibrary.FindLookAtRotation` _returnvalue (`self.K2_GetActorLocation` (`self.Player`)))) -10))) (.y (+ _returnvalue (* (`KismetMathLibrary.GetForwardVector` (`KismetMathLibrary.FindLookAtRotation` _returnvalue (`self.K2_GetActorLocation` (`self.Player`)))) -10))) (.z _returnvalue)) null
    (:`then`
      (bind _true (`self.Objects Around`))
      (if _true
        (`self.Attack`)))))

(event `Attack`
  (bind _cube (`self.Cube`))
  (bind _capsulecomponent (`self.CapsuleComponent`))
  (bind (_returnvalue_roll _returnvalue_pitch _returnvalue_yaw) (`KismetMathLibrary.BreakRotator` (`SceneComponent.K2_GetComponentRotation` _cube)))
  (if (not (`self.Attacking`))
    (switch `int` (`self.Type`)
      (:`0`
        (bind _output (`self.Check if sight is Blocked`))
        (if (not _output)
          (set `self.Attacking` true)
          (`ActorComponent.SetActive` (`self.CharacterMovement`) false false)
          (`self.Look At Player`)
          (bind (_direction _turn) (`Timeline|Timeline_0` :!via `PlayFromStart`)
            (:`Update`
              (`SceneComponent.K2_SetWorldRotation` _cube (`KismetMathLibrary.MakeRotator` _turn _returnvalue_pitch _returnvalue_yaw) false false))
            (:`Finished`
              (`KismetSystemLibrary.Delay` 0.5)
              (if (`self.Player In Attacking Range`)
                (bind _astop_down_character (cast `/Game/TopDownBP/Blueprints/TopDownCharacter` (`self.Player`)))
                (`/Game/TopDownBP/Blueprints/TopDownCharacter.Hit` _astop_down_character 10.0)
                (set `self.Attacking` false)
                (`self.Attack`)
                (else
                  (set `self.Attacking` false)
                  (`ActorComponent.SetActive` (`self.CharacterMovement`) true false)))))))
      (:`1`
        (bind _output_2 (`self.Check if sight is Blocked`))
        (if (not _output_2)
          (set `self.Attacking` true)
          (`ActorComponent.SetActive` (`self.CharacterMovement`) false false)
          (`self.Look At Player`)
          (`MovementComponent.StopMovementImmediately` (`self.CharacterMovement`))
          (`KismetSystemLibrary.Delay` 0.2)
          (`|SpawnActorFromClass` "/Game/_MyContent/BluePrints/Enemy_Laser.Enemy_Laser_C" (`KismetMathLibrary.MakeTransform` (`SceneComponent.K2_GetComponentLocation` _capsulecomponent) (`SceneComponent.K2_GetComponentRotation` _capsulecomponent) (2.0 2.0 2.0)) "Undefined" "OverrideRootScale" null null)
          (`KismetSystemLibrary.Delay` 1.0)
          (set `self.Attacking` false)
          (`ActorComponent.SetActive` (`self.CharacterMovement`) true false)))
      (:`2`
        (`self.Healer Attack`))
      (:`3`
        (`self.Sapling Attack`))
      (:`4`
        (`self.Spawner Attack`)))))

(event `Healer Attack`
  (set `self.Attacking` true)
  (`ActorComponent.SetActive` (`self.CharacterMovement`) false false)
  (`self.Look At Player`)
  (`self.Heal Nearby Enemies`)
  (bind _returnvalue (`AddComponent|NODE_AddStaticMeshComponent-1` :`RelativeTransform` (`KismetMathLibrary.MakeTransform` (0.0 0.0 -80.0) (struct) (2.0 2.0 0.1))))
  (`StaticMeshComponent.SetStaticMesh` _returnvalue "/Game/_MyContent/Models/Healer_Circle.Healer_Circle")
  (`PrimitiveComponent.SetCollisionEnabled` _returnvalue "NoCollision")
  (`PrimitiveComponent.SetMaterial` _returnvalue 0 "/Game/_MyContent/Materials/Gold_Glow.Gold_Glow")
  (bind (_direction _height) (`Timeline|Healing Effect` :!via `PlayFromStart`)
    (:`Update`
      (`SceneComponent.K2_SetRelativeLocation` _returnvalue (`KismetMathLibrary.MakeVector` 0.0 0.0 _height) false false))
    (:`Finished`
      (`ActorComponent.K2_DestroyComponent` _returnvalue)
      (`KismetSystemLibrary.Delay` 0.5)
      (set `self.Attacking` false)
      (`ActorComponent.SetActive` (`self.CharacterMovement`) true false))))

(event `Sapling Attack`
  (bind _cube (`self.Cube`))
  (set `self.Attacking` true)
  (`PrimitiveComponent.SetCollisionEnabled` (`self.CapsuleComponent`) "NoCollision")
  (`ActorComponent.SetActive` (`self.CharacterMovement`) false false)
  (`self.Look At Player`)
  (bind (_direction _rotation _movement) (`Timeline|Dive` :!via `PlayFromStart`)
    (:`Update`
      (`SceneComponent.K2_SetRelativeRotation` _cube (`KismetMathLibrary.MakeRotator` _rotation 0.0 -90.0) false false)
      (`SceneComponent.K2_SetRelativeLocation` _cube (`KismetMathLibrary.MakeVector` _movement 0.0 -40.0) false false))
    (:`Finished`
      (if (`self.Player In Attacking Range`)
        (bind _astop_down_character (cast `/Game/TopDownBP/Blueprints/TopDownCharacter` (`self.Player`)))
        (`/Game/TopDownBP/Blueprints/TopDownCharacter.Hit` _astop_down_character 5.0))
      (`self.K2_DestroyActor`))))

(event `Spawner Attack`
  (`ActorComponent.SetActive` (`self.CharacterMovement`) false false)
  (set `self.Attacking` true)
  (bind _returnvalue (`AIBlueprintHelperLibrary.SpawnAIFromClass` "Enemy_C" null (`SceneComponent.K2_GetComponentLocation` (`self.Spawner 1`)) (struct) false null))
  (bind _asenemy (cast `/Game/_MyContent/BluePrints/Enemy` _returnvalue))
  (set `/Game/_MyContent/BluePrints/Enemy.Type` 3 _asenemy)
  (`self.Set Type` _asenemy)
  (bind _returnvalue_2 (`AIBlueprintHelperLibrary.SpawnAIFromClass` "Enemy_C" null (`SceneComponent.K2_GetComponentLocation` (`self.Spawner 2`)) (struct) false null))
  (bind _asenemy_2 (cast `/Game/_MyContent/BluePrints/Enemy` _returnvalue_2))
  (set `/Game/_MyContent/BluePrints/Enemy.Type` 3 _asenemy_2)
  (`self.Set Type` _asenemy_2)
  (`KismetSystemLibrary.Delay` 2.5)
  (set `self.Attacking` false)
  (`ActorComponent.SetActive` (`self.CharacterMovement`) true false))

(fn `Check if sight is Blocked`
  (returns (Output :type Boolean))
  (bind (_outhit _returnvalue) (`KismetSystemLibrary.LineTraceSingle` (`SceneComponent.K2_GetComponentLocation` (`self.Mesh`)) (`SceneComponent.K2_GetComponentLocation` (`Actor.RootComponent` (`self.Player`))) "TraceTypeQuery1" false (`|MakeArray` self :!type "Actor Object Reference")))
  (`KismetSystemLibrary.PrintString` (`KismetSystemLibrary.GetDisplayName` (`.HitActor` (`GameplayStatics.BreakHitResult` _outhit))))
  (return _returnvalue))

(fn `Damage`
  (params (Amount :type "Float (double-precision)"))
  (bind _health (`self.Health`))
  (set `self.Health` (- _health Amount))
  (set `/Game/_MyContent/UI/HealthBar.Health Percent` (/ _health (`self.Starting Health`)) (`self.Health Bar`))
  (if (<= (`self.Health`) 0.0)
    (`self.K2_DestroyActor`)))

(fn `Heal`
  (params (Amount :type "Float (double-precision)"))
  (bind _health (`self.Health`))
  (set `self.Health` (+ _health Amount))
  (set `/Game/_MyContent/UI/HealthBar.Health Percent` (/ _health (`self.Starting Health`)) (`self.Health Bar`))
  (if (>= (`self.Health`) (`self.Starting Health`))
    (set `self.Health` (`self.Starting Health`))))

(fn `Heal Nearby Enemies`
  (bind _overlappingactors (`PrimitiveComponent.GetOverlappingActors` (`self.Healing Range`) "Enemy_C"))
  (if (!= (`KismetArrayLibrary.Array_Length` _overlappingactors) 0)
    (for _array_element _overlappingactors
      (bind _asenemy (cast `/Game/_MyContent/BluePrints/Enemy` _array_element))
      (`self.Heal` _asenemy 150.0))))

(fn `Look At Player`
  (bind (_returnvalue_roll _returnvalue_pitch) (`KismetMathLibrary.BreakRotator` (`SceneComponent.K2_GetComponentRotation` (`self.CapsuleComponent`))))
  (bind (_returnvalue_roll_2 _returnvalue_pitch_2 _returnvalue_yaw) (`KismetMathLibrary.BreakRotator` (`KismetMathLibrary.FindLookAtRotation` (`SceneComponent.K2_GetComponentLocation` (`self.Mesh`)) (`SceneComponent.K2_GetComponentLocation` (`Actor.RootComponent` (`self.Player`))))))
  (`SceneComponent.K2_SetWorldRotation` (`self.CapsuleComponent`) (`KismetMathLibrary.MakeRotator` _returnvalue_roll _returnvalue_pitch _returnvalue_yaw) false false))

(fn `Objects Around`
  (returns (True :type Boolean))
  (locals (NewLocalVar_1 :type "Array of Actor Class Reference"))
  (return (!= (`KismetArrayLibrary.Array_Length` (`PrimitiveComponent.GetOverlappingActors` (`self.Path Detection`) "/Game/_MyContent/BluePrints/Wall.Wall_C")) 0)))

(fn `Set Random Type`
  (locals (X :type "Float (double-precision)") (`Type Chance` :type "Array of Float (double-precision)"))
  (bind _x (`local.X`))
  (bind _output (`|GetArrayItem` (`local.Type Chance`)))
  (bind _returnvalue (+ _output (`|GetArrayItem` (`local.Type Chance`) 1)))
  (bind _output_get (set `local.X` 74.0))
  (`KismetSystemLibrary.PrintString` (`KismetStringLibrary.Conv_DoubleToString` _output_get))
  (if (`KismetMathLibrary.InRange_FloatFloat` _x 0.0 _output)
    (`KismetSystemLibrary.PrintString` "0")
    (set `self.Type` 0)
    (elif (`KismetMathLibrary.InRange_FloatFloat` _x _output _returnvalue)
      (`KismetSystemLibrary.PrintString` "1")
      (set `self.Type` 1)
      (elif (`KismetMathLibrary.InRange_FloatFloat` _x _returnvalue (+ _returnvalue (`|GetArrayItem` (`local.Type Chance`) 2)))
        (`KismetSystemLibrary.PrintString` "2")
        (set `self.Type` 2)
        (else
          (`KismetSystemLibrary.PrintString` "3")
          (set `self.Type` 4)))))
  (`self.Set Type`))

(fn `Set Type`
  (bind _cube (`self.Cube`))
  (switch `int` (`self.Type`)
    (:`0`
      (set `self.Attacking Range` 75.0)
      (`StaticMeshComponent.SetStaticMesh` (`self.Cube`) "/Game/_MyContent/Models/Skeleton.Skeleton" :!label _label))
    (:`1`
      (goto _label))
    (:`2`
      (set `self.Attacking Range` 300.0 :!label _label_2)
      (set `self.Running Range` 200.0)
      (`StaticMeshComponent.SetStaticMesh` _cube "/Game/_MyContent/Models/Healer.Healer"))
    (:`3`
      (`StaticMeshComponent.SetStaticMesh` (`self.Cube`) "/Game/Geometry/Meshes/1M_Cube.1M_Cube")
      (set `self.Attacking Range` 200.0)
      (`SceneComponent.SetRelativeScale3D` _cube (0.5 0.5 0.5))
      (`SceneComponent.K2_SetRelativeLocation` _cube (0.0 0.0 -40.0) false false)
      (set `CharacterMovementComponent.MaxWalkSpeed` 450.0 (`self.CharacterMovement`))
      (`Widget.SetVisibility` (`self.Health Bar`) "Hidden"))
    (:`4`
      (goto _label_2)))
  (set `self.Health` (`self.Starting Health`)))

(fn `UserConstructionScript`
  (locals (X :type "Float (double-precision)") (`Type Chance` :type "Array of Float (double-precision)"))
  (`KismetSystemLibrary.PrintString` "Construct")
  (if (== (`self.Type`) -1)
    (`self.Set Random Type`))
  (`self.Set Type`))