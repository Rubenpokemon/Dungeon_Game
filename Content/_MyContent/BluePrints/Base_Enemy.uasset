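; Base enemy for a top-down game that chases the player with AI MoveTo and attacks by melee or laser, with a health bar widget.
; Type selects which sight component survives construction, currently hard-set to ranged.
; Ranged enemies stop to fire Enemy_Laser every second, back away when the player is close and resume chasing beyond range.
; Melee enemies play a timeline spin, hitting while overlap persists; Damage destroys the enemy at zero health.
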(event `self.ReceiveBeginPlay`
  (`|ExecutionSequence`
    (:`then_0`
      (`KismetSystemLibrary.Delay` 0.2)
      (if (`self.Moving Forward`) :!label _label
        (`|AIMoveTo` self (`self.K2_GetActorLocation` (`GameplayStatics.GetPlayerPawn` 0)) null
          (:`OnSuccess`
            _))
        (else
          (`self.Run Away`)))
      (`KismetSystemLibrary.Delay` 0.2)
      (`KismetSystemLibrary.PrintString` "Movement Loop")
      (goto _label))
    (:`then_1`
      (bind _ashealth_bar (cast `/Game/_MyContent/UI/HealthBar` (`WidgetComponent.GetUserWidgetObject` (`self.Widget`))))
      (bind _output_get (set `self.Health Bar` _ashealth_bar))
      (set `/Game/_MyContent/UI/HealthBar.Health Percent` 1.0 _output_get))))

(event `self.Melee Sight.OnComponentBeginOverlap`
  (params (OverlappedComponent :type "PrimitiveComponent Object Reference") (OtherActor :type "Actor Object Reference") (OtherComp :type "PrimitiveComponent Object Reference") (OtherBodyIndex :type Integer) (bFromSweep :type Boolean) (SweepResult :type "HitResult Structure (by ref)"))
  (bind (_returnvalue_roll _returnvalue_pitch _returnvalue_yaw) (`KismetMathLibrary.BreakRotator` (`SceneComponent.K2_GetComponentRotation` (`self.Mesh`))))
  (bind _astop_down_character (cast `/Game/TopDownBP/Blueprints/TopDownCharacter` OtherActor))
  (set `self.Player` _astop_down_character)
  (`ActorComponent.SetActive` (`self.CharacterMovement`) false false)
  (bind (_direction _turn) (`Timeline|Melee Attack` :!via `PlayFromStart` :!label _label_2)
    (:`Update`
      (`SceneComponent.K2_SetWorldRotation` (`self.Mesh`) (`KismetMathLibrary.MakeRotator` _turn _returnvalue_pitch _returnvalue_yaw) false false))
    (:`Finished`
      (if (== (`KismetArrayLibrary.Array_Length` (`PrimitiveComponent.GetOverlappingActors` (`self.Melee Sight`) "/Game/TopDownBP/Blueprints/TopDownCharacter.TopDownCharacter_C")) 1)
        (`/Game/TopDownBP/Blueprints/TopDownCharacter.Hit` (`self.Player`) (`self.Melee Damage`))
        (goto _label_2 :!via `PlayFromStart`)
        (else
          (`ActorComponent.SetActive` (`self.CharacterMovement`) true false))))))

(event `self.Ranged Sight.OnComponentBeginOverlap`
  (params (OverlappedComponent :type "PrimitiveComponent Object Reference") (OtherActor :type "Actor Object Reference") (OtherComp :type "PrimitiveComponent Object Reference") (OtherBodyIndex :type Integer) (bFromSweep :type Boolean) (SweepResult :type "HitResult Structure (by ref)"))
  (bind _charactermovement (`self.CharacterMovement`))
  (bind _capsulecomponent (`self.CapsuleComponent`))
  (bind _astop_down_character (cast `/Game/TopDownBP/Blueprints/TopDownCharacter` OtherActor))
  (set `self.Player` _astop_down_character)
  (if (`ActorComponent.IsActive` _charactermovement)
    (`ActorComponent.SetActive` _charactermovement false false)
    (set `self.Player In Sight` true)
    (`self.Look at Player` :!label _label_3)
    (`|SpawnActorFromClass` "/Game/_MyContent/BluePrints/Enemy_Laser.Enemy_Laser_C" (`KismetMathLibrary.MakeTransform` (`SceneComponent.K2_GetComponentLocation` _capsulecomponent) (`SceneComponent.K2_GetComponentRotation` _capsulecomponent) (2.0 2.0 2.0)) "Undefined" "OverrideRootScale" null null)
    (`KismetSystemLibrary.Delay` 1.0)
    (bind _output_get (set `self.Distance To Player` (`KismetMathLibrary.VSize` (- (`self.K2_GetActorLocation` (`self.Player`)) (`SceneComponent.K2_GetComponentLocation` (`self.CapsuleComponent`))))))
    (`KismetSystemLibrary.PrintString` (`KismetStringLibrary.Conv_DoubleToString` _output_get))
    (if (<= _output_get 300.0)
      (`ActorComponent.SetActive` (`self.CharacterMovement`) true false)
      (`self.Run Away`)
      (elif (`KismetMathLibrary.InRange_FloatFloat` _output_get 301.0 500.0)
        (goto _label_3)
        (else
          (`KismetSystemLibrary.PrintString` "Move Foward")
          (set `self.Moving Forward` true)
          (`ActorComponent.SetActive` (`self.CharacterMovement`) true false)
          (`|AIMoveTo` self (`self.K2_GetActorLocation` (`GameplayStatics.GetPlayerPawn` 0)) null))))))

(event `Run Away`
  (bind _returnvalue (`self.K2_GetActorLocation`))
  (bind _returnvalue_2 (`KismetMathLibrary.VSize` (- (`self.K2_GetActorLocation` (`self.Player`)) (`SceneComponent.K2_GetComponentLocation` (`self.CapsuleComponent`)))))
  (`|AIMoveTo` self (`KismetMathLibrary.MakeVector` (.x (+ _returnvalue (* (`KismetMathLibrary.GetForwardVector` (`KismetMathLibrary.FindLookAtRotation` _returnvalue (`self.K2_GetActorLocation` (`self.Player`)))) -100))) (.y (+ _returnvalue (* (`KismetMathLibrary.GetForwardVector` (`KismetMathLibrary.FindLookAtRotation` _returnvalue (`self.K2_GetActorLocation` (`self.Player`)))) -100))) (.z _returnvalue)) null
    (:`OnSuccess`
      _)
    (:`OnFail`
      _))
  (if (>= _returnvalue_2 300.0)
    (set `self.Moving Forward` true)
    (`KismetSystemLibrary.PrintString` "Stop Running")
    (if (`KismetMathLibrary.InRange_FloatFloat` _returnvalue_2 301.0 500.0)
      (goto _label_3)
      (else
        (`|AIMoveTo` self (`self.K2_GetActorLocation` (`GameplayStatics.GetPlayerPawn` 0)) null)))
    (else
      (`self.Run Away`))))

(fn `Damage`
  (params (Amount :type "Float (double-precision)"))
  (bind _health (`self.Health`))
  (set `self.Health` (- _health Amount))
  (set `/Game/_MyContent/UI/HealthBar.Health Percent` (/ _health (`self.Starting Health`)) (`self.Health Bar`))
  (if (<= (`self.Health`) 0.0)
    (`self.K2_DestroyActor`)))

(fn `Look at Player`
  (bind (_returnvalue_roll _returnvalue_pitch) (`KismetMathLibrary.BreakRotator` (`SceneComponent.K2_GetComponentRotation` (`self.CapsuleComponent`))))
  (bind (_returnvalue_roll_2 _returnvalue_pitch_2 _returnvalue_yaw) (`KismetMathLibrary.BreakRotator` (`KismetMathLibrary.FindLookAtRotation` (`SceneComponent.K2_GetComponentLocation` (`self.Mesh`)) (`SceneComponent.K2_GetComponentLocation` (`Character.Mesh` (`self.Player`))))))
  (`SceneComponent.K2_SetWorldRotation` (`self.CapsuleComponent`) (`KismetMathLibrary.MakeRotator` _returnvalue_roll _returnvalue_pitch _returnvalue_yaw) false false))

(fn `Set Type`
  (switch `int` (`self.Type`)
    (:`0`
      (`ActorComponent.K2_DestroyComponent` (`self.Ranged Sight`)))
    (:`1`
      (`ActorComponent.K2_DestroyComponent` (`self.Melee Sight`)))))

(fn `UserConstructionScript`
  (locals (NewLocalVar_0 :type "Array of Name"))
  (set `self.Type` 1)
  (`self.Set Type`)
  (set `CharacterMovementComponent.MaxWalkSpeed` (`self.Speed`) (`self.CharacterMovement`))
  (set `self.Health` (`self.Starting Health`))
  (set `self.Tags` (`local.NewLocalVar_0`)))