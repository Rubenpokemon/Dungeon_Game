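; ControlPoint is a capture point that the TopDownCharacter takes by staying inside its scalable Area, while enemies spawn.
; Overlap starts two self-repeating delayed event loops that run while the player remains inside.
; One lowers the Flag, turns it pink, then raises it until capture completes and the Area is destroyed.
; The other spawns AI enemies at shuffled SpawnPoints after random intervals.
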(event `self.Area.OnComponentBeginOverlap`
  (params (OverlappedComponent :type "PrimitiveComponent Object Reference") (OtherActor :type "Actor Object Reference") (OtherComp :type "PrimitiveComponent Object Reference") (OtherBodyIndex :type Integer) (bFromSweep :type Boolean) (SweepResult :type "HitResult Structure (by ref)"))
  (cast `/Game/TopDownBP/Blueprints/TopDownCharacter` OtherActor)
  (`self.Start Caputure`)
  (`self.Spawn Enemies`))

(event `Start Caputure`
  (if (not (`self.Done`))
    (`KismetSystemLibrary.Delay` 0.01)
    (if (`self.Player In Area`)
      (`self.Move Flag`)
      (`self.Start Caputure`))))

(event `Spawn Enemies`
  (`KismetSystemLibrary.Delay` (`KismetMathLibrary.RandomFloatInRange` 2.5 3.5))
  (if (`KismetSystemLibrary.IsValid` (`self.Area`))
    (if (`self.Player In Area`)
      (`self.Spawn Enemy`)
      (`self.Spawn Enemies`))))

(fn `Move Flag`
  (bind _flag (`self.Flag`))
  (bind _flag_2 (`self.Flag`))
  (bind (_relativelocation_x _relativelocation_y _relativelocation_z) (`KismetMathLibrary.BreakVector` (`SceneComponent.RelativeLocation` _flag)))
  (bind (_relativelocation_x_2 _relativelocation_y_2 _relativelocation_z_2) (`KismetMathLibrary.BreakVector` (`SceneComponent.RelativeLocation` _flag_2)))
  (if (`self.Moving Down`)
    (`SceneComponent.K2_SetRelativeLocation` _flag_2 (`KismetMathLibrary.MakeVector` _relativelocation_x_2 _relativelocation_y_2 (- _relativelocation_z_2 (`self.Flag Speed`))) false false)
    (if (<= _relativelocation_z_2 0.0)
      (set `self.Moving Down` false)
      (`PrimitiveComponent.SetMaterial` (`self.Flag`) 0 "/Game/_MyContent/Materials/Pink.Pink"))
    (else
      (`SceneComponent.K2_SetRelativeLocation` _flag (`KismetMathLibrary.MakeVector` _relativelocation_x _relativelocation_y (+ _relativelocation_z (`self.Flag Speed`))) false false)
      (if (>= _relativelocation_z 300.0)
        (set `self.Done` true)
        (`ActorComponent.K2_DestroyComponent` (`self.Area`))))))

(fn `Spawn Enemy`
  (`KismetArrayLibrary.Array_Shuffle` (`self.Spawn Points`))
  (`AIBlueprintHelperLibrary.SpawnAIFromClass` "/Game/_MyContent/BluePrints/Enemy.Enemy_C" null (`SceneComponent.K2_GetComponentLocation` (`Actor.RootComponent` (`|GetArrayItem` (`self.Spawn Points`)))) (struct) true null))

(fn `UserConstructionScript`
  (bind _area_scale (`self.Area Scale`))
  (`SceneComponent.SetRelativeScale3D` (`self.Area`) (`KismetMathLibrary.MakeVector` _area_scale _area_scale 0.1)))